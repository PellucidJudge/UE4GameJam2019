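; Energy capsule pickup that drifts out when released, then homes in on the player and grants energy through BP_PlayerController.
; ReleaseCapsule uses a timeline to move it along the given direction at a random speed set on BeginPlay, then enables seeking.
; Tick lerps it toward the player character by delta time while seeking, and within the proximity threshold adds energy and destroys the capsule.
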(event Custom|ReleaseCapsule
  (params (StartTravelDir :type Vector))
  (Variables|Default|SetStartTravelDir StartTravelDir)
  (bind _newtrack_0 (Timeline|StartTimeline PlayFromStart)
    (:Update
      (Transformation|SetActorLocation (+ (Transformation|GetActorLocation) (* (* (* (Variables|Default|GetStartTravelDir) (Utilities|Time|GetWorldDeltaSeconds)) (Variables|Default|GetFloatingSpeed)) _newtrack_0)) false false))
    (:Finished
      (Variables|Default|SetIsSeekingPlayer true))))

(event EventBeginPlay
  (bind _returnvalue (Game|GetPlayerCharacter 0))
  (Utilities|IsValid _returnvalue
    (:Is%20Valid
      (Variables|Default|SetPlayerCharacterRef _returnvalue)
      (Variables|Default|SetFloatingSpeed (Math|Random|RandomFloatinRange 5e+01 2.5e+02)))
    (:Is%20Not%20Valid
      (Actor|DestroyActor))))

(event EventTick
  (params (DeltaSeconds :type Float%20%28single-precision%29))
  (bind _returnvalue (Game|GetPlayerController 0))
  (bind _playercharacterref (Variables|Default|GetPlayerCharacterRef))
  (Utilities|IsValid _playercharacterref
    (:Is%20Valid
      (if (< (Math|Vector|VectorLength (- (Transformation|GetActorLocation _playercharacterref) (Transformation|GetActorLocation))) (Variables|Default|GetNeededProximity))
        (Utilities|IsValid _returnvalue
          (:Is%20Valid
            (bind _asbp_player_controller (Utilities|Casting|CastToBP_PlayerController _returnvalue))
            (Default|AddEnergy _asbp_player_controller (Variables|Default|GetEnergyAmount))
            (Actor|DestroyActor)))
        (elif (Variables|Default|GetIsSeekingPlayer)
          (Transformation|SetActorLocation (Math|Vector|Lerp(Vector) (Transformation|GetActorLocation) (Transformation|GetActorLocation (Variables|Default|GetPlayerCharacterRef)) DeltaSeconds) false false))))))

(fn ConstructionScript)