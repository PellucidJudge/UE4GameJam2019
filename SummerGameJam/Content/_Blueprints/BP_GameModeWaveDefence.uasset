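; Wave defence game mode that cycles through preparation, assault, extermination, cooldown and an optional shop phase, currently a pass-through.
; Each wave's DT_Waves row, keyed by wave number, sets enemies queued at random spawn points and feeds the HUD widget.
; Tick ends the assault once all spawners finish and no tracked enemies remain.
; Timelines time preparation and cooldown; a missing row ends the game with a printed message.
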(event Custom|GetPlayer
  (bind _asbp_player_character (Utilities|Casting|CastToBP_PlayerCharacter (Game|Player|GetPlayerPawn 0)))
  (Variables|Default|SetPlayerCharacter _asbp_player_character))

(event Custom|StartGame
  ;[1 1 1] Phases
  ;;[0 0.01254 0.09375] Start Game
  (CallFunction|SwitchPhase "NewEnumerator0" "NewEnumerator0")
  (CallFunction|StartPhasePreparation))

(event Custom|AddWaveDataWidget
  (Utilities|IsValid (Variables|Default|GetWaveDataDisplay)
    (:Is%20Not%20Valid
      (bind _returnvalue (UserInterface|CreateWidget "/Game/_Blueprints/UI/HUD/W_WaveDataDisplay.W_WaveDataDisplay_C"))
      (bind _output_get (Variables|Default|SetWaveDataDisplay _returnvalue))
      (UserInterface|Viewport|AddtoViewport _output_get 0))))

(event Custom|SwitchPhase
  (params (NewPhase :type E_GamePhases%20Enum :default "NewEnumerator0") (OldPhase :type E_GamePhases%20Enum :default "NewEnumerator0"))
  (bind _wavedatadisplay (Variables|Default|GetWaveDataDisplay))
  (Utilities|IsValid _wavedatadisplay
    (:Is%20Valid
      (bind _returnvalue (Utilities|GetDataTableRow "/Game/_Blueprints/DataTables/DT_Waves.DT_Waves" (Utilities|String|StringToName (Utilities|String|ToString(Integer) (Variables|Default|GetCurrentWave))))
        (:then
          (Default|UpdateDisplay _wavedatadisplay _returnvalue NewPhase))))))

(event Custom|StartPhase_Preparation
  ;[1 1 1] Phases
  ;;[0 0.01254 0.09375] PrepPhase
  (Variables|Default|SetMode "NewEnumerator0")
  (Timeline|PreparationTimeline PlayFromStart
    (:Finished
      (CallFunction|SwitchPhase "NewEnumerator0" "NewEnumerator1")
      (CallFunction|StartPhaseWaveAssault))))

(event Custom|StartPhase_WaveAssault
  ;[1 1 1] Phases
  ;;[0 0.01254 0.09375] Wave assault
  (CallFunction|ResetSpawners)
  (bind _returnvalue (Utilities|GetDataTableRow "/Game/_Blueprints/DataTables/DT_Waves.DT_Waves" (Utilities|String|StringToName (Utilities|String|ToString(Integer) (Variables|Default|GetCurrentWave))))
    (:then
      (CallFunction|SpawnWave _returnvalue)
      (CallFunction|PrimeSpawners)
      (Variables|Default|SetMode "NewEnumerator1"))
    (:RowNotFound
      (CallFunction|FinishGame))))

(event Custom|StartPhase_Extermination
  ;[1 1 1] Phases
  ;;[0 0.01254 0.09375] Extermination
  (Variables|Default|SetMode "NewEnumerator2")
  (for _array_element (Variables|Default|GetEnemies)
    (Actor|DestroyActor _array_element))
  (Utilities|Array|Clear (Variables|Default|GetEnemies))
  (CallFunction|SwitchPhase "NewEnumerator2" "NewEnumerator3")
  (CallFunction|StartPhaseCooldown))

(event Custom|StartPhase_Cooldown
  ;[1 1 1] Phases
  ;;[0 0.01254 0.09375] Cooldown
  (Variables|Default|SetMode "NewEnumerator3")
  (Timeline|CooldownPhaseTimeline PlayFromStart
    (:Finished
      (bind _returnvalue (Utilities|GetDataTableRow "/Game/_Blueprints/DataTables/DT_Waves.DT_Waves" (Utilities|String|StringToName (Utilities|String|ToString(Integer) (Variables|Default|GetCurrentWave))))
        (:then
          (if (.Shop (Utilities|Struct|BreakS_WaveData _returnvalue))
            (CallFunction|SwitchPhase "NewEnumerator3" "NewEnumerator4")
            (CallFunction|StartPhaseShop)
            (else
              (CallFunction|SwitchPhase "NewEnumerator3" "NewEnumerator0")
              (CallFunction|FinishWave))))
        (:RowNotFound
          (CallFunction|FinishGame))))))

(event Custom|StartPhase_Shop
  ;[1 1 1] Phases
  ;;[0 0.01254 0.09375] Shop
  (Variables|Default|SetMode "NewEnumerator3")
  (CallFunction|FinishWave))

(event Custom|FinishWave
  ;[1 1 1] Phases
  ;;[0 0.01254 0.09375] Finish wave
  (Math|Integer|IncrementInt (Variables|Default|GetCurrentWave)
    (:%20%20
      (CallFunction|StartPhasePreparation))))

(event Custom|FinishGame
  ;[1 1 1] Finish
  (Development|PrintString "CONGRATS"))

(event Custom|SpawnerDone
  (Math|Integer|IncrementInt (Variables|Default|GetFinishedSpawnerCount)))

(event EventBeginPlay
  (bind _outactors (Actor|GetAllActorsOfClass "/Game/_Blueprints/WaveSystem/BP_WaveSpawnPoint.BP_WaveSpawnPoint_C"))
  (Variables|Default|SetSpawnPoints _outactors)
  (CallFunction|GetPlayer)
  (CallFunction|StartGame)
  (CallFunction|AddWaveDataWidget))

(event EventTick
  (params (DeltaSeconds :type Float%20%28single-precision%29))
  ;[1 1 1] Tick
  (Utilities|FlowControl|Sequence
    (:then_1
      ;;[0 0.01254 0.09375] Phase logic
      (switch Utilities|FlowControl|Switch|SwitchonE_GamePhases (Variables|Default|GetMode)
        (:NewEnumerator1
          (if (<= (Utilities|Array|Length (Variables|Default|GetEnemies)) 0)
            ;;;[1 1 1] Check if all enemies have spawned
            (if (>= (Variables|Default|GetFinishedSpawnerCount) (Utilities|Array|Length (Variables|Default|GetSpawnPoints)))
              (CallFunction|SwitchPhase "NewEnumerator1" "NewEnumerator2")
              (CallFunction|StartPhaseExtermination))))))))

(fn ConstructionScript)

(fn SpawnWave
  (params (WaveData :type S%20Wave%20Data%20Structure))
  (bind (_wavenumber _wavename _shop _enemytypes _numberofenemies) (Utilities|Struct|BreakS_WaveData WaveData))
  (for (_array_element _array_index) _enemytypes
    (if (and (Utilities|IsValidClass _array_element) (Utilities|Array|IsValidIndex _numberofenemies _array_index))
      (for _index (range 1 (Utilities|Array|Get(acopy) _numberofenemies _array_index))
        (Default|SpawnEnemy (Utilities|Array|Get(acopy) (Variables|Default|GetSpawnPoints) (Math|Random|RandomIntegerinRange 0 (Math|Integer|Max(Integer) (- (Utilities|Array|Length (Variables|Default|GetSpawnPoints)) 1)))) _array_element)))))

(fn AddEnemy
  (params (Enemy :type BP%20Enemy%20Base%20Object%20Reference))
  (Utilities|Array|AddUnique (Variables|Default|GetEnemies) Enemy))

(fn PrimeSpawners
  (Variables|Default|SetFinishedSpawnerCount 0)
  (for _array_element (Variables|Default|GetSpawnPoints)
    (Default|PrimeSpawnpoint _array_element)))

(fn ResetSpawners
  (for _array_element (Variables|Default|GetSpawnPoints)
    (Default|Reset _array_element)))

(fn EnemyDeath
  (params (Enemy :type BP%20Enemy%20Base%20Object%20Reference))
  (Utilities|Array|RemoveItem (Variables|Default|GetEnemies) Enemy))