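; BP_DestrucibleObject is a destructible environment object with a health pool that removes itself from the world when depleted.
; Health starts at MaxHealth on BeginPlay, then HealthDamage lowers it to a floor of zero and fires Destroyed, which simply destroys the actor.
; HealthHeal restores health up to the maximum, only when CanBeHealed is set.
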(event Custom|Destroyed
  (Actor|DestroyActor))

(event EventHealthDamage
  (params (Amount :type Float%20%28single-precision%29) (Instigator :type Actor%20Object%20Reference) (DamageType :type Damage%20Type%20Class%20Reference))
  (bind _output_get (Variables|Default|SetCurrentHealth (Math|Float|Max(Float) (- (Variables|Default|GetCurrentHealth) Amount) 0.0)))
  (if (<= _output_get 0.0)
    (CallFunction|Destroyed)))

(event EventHealthHeal
  (params (Amount :type Float%20%28single-precision%29) (Instigator :type Actor%20Object%20Reference))
  (if (Variables|Default|GetCanBeHealed)
    (Variables|Default|SetCurrentHealth (Math|Float|Min(Float) (+ (Variables|Default|GetCurrentHealth) Amount) (Variables|Default|GetMaxHealth)))))

(event EventBeginPlay
  (Variables|Default|SetCurrentHealth (Variables|Default|GetMaxHealth)))

(fn ConstructionScript)