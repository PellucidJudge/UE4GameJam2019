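; A spawn point actor for the wave defence game mode that creates enemies at its own location.
; SpawnEnemy spawns the given enemy class unrotated at the actor's position and, if valid, registers it with BP_GameModeWaveDefence through AddEnemy.
; PrimeSpawnpoint does no setup of its own and immediately reports SpawnerDone to the game mode.
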(event Custom|SpawnEnemy
  (params (EnemyClass :type BP%20Enemy%20Base%20Class%20Reference))
  (bind _asbp_game_mode_wave_defence (Utilities|Casting|CastToBP_GameModeWaveDefence (Game|GetGameMode)))
  (bind _returnvalue (Game|SpawnActorfromClass EnemyClass (Math|Transform|MakeTransform (Transformation|GetActorLocation)) "Undefined" 0 0))
  (Utilities|IsValid _returnvalue
    (:Is%20Valid
      (Default|AddEnemy _asbp_game_mode_wave_defence _returnvalue))))

(event Custom|Reset)

(event Custom|PrimeSpawnpoint
  (bind _asbp_game_mode_wave_defence (Utilities|Casting|CastToBP_GameModeWaveDefence (Game|GetGameMode)))
  (Default|SpawnerDone _asbp_game_mode_wave_defence))

(event EventBeginPlay)

(event Collision|EventActorBeginOverlap
  (params (OtherActor :type Actor%20Object%20Reference)))

(event EventTick
  (params (DeltaSeconds :type Float%20%28single-precision%29)))

(fn ConstructionScript)