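; Base AI controller for melee enemies that target the player and attack at close range.
; BeginPlay runs the melee behavior tree and blackboard, storing the player pawn as target.
; While the controlled character lives, Tick feeds the player's location to the blackboard's WantedPosition.
; Attacks bypass the tree: Tick calls the character's Attack1 when the target is in range and the cooldown, not decremented here, has expired.
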(event Custom|MakeMeleeAttack
  (params (AimLocation :type Vector))
  (bind _controlledchar (Variables|Default|GetControlledChar))
  (Utilities|IsValid _controlledchar
    (:Is%20Valid
      (Default|Attack1 _controlledchar))))

(event EventBeginPlay
  (bind _returnvalue (AI|GetBlackboard 0))
  (bind _returnvalue_2 (Game|Player|GetPlayerPawn 0))
  (|CallParentFunction)
  (Class|AIController|UseBlackboard "/Game/_Blueprints/AI/BB_MeleeEnemy.BB_MeleeEnemy")
  (AI|RunBehaviorTree "/Game/_Blueprints/AI/BT_MeleeEnemy.BT_MeleeEnemy")
  (Utilities|IsValid _returnvalue_2
    (:Is%20Valid
      (Variables|Default|SetTarget _returnvalue_2)
      (Utilities|IsValid _returnvalue
        (:Is%20Valid
          (AI|Components|Blackboard|SetValueasObject _returnvalue (Utilities|Name|MakeLiteralName (Variables|Default|GetBBKey_Target)) _returnvalue_2))
        (:Is%20Not%20Valid
          (Development|PrintString "Error: Invalid Blackboard" true true "(R=1.000000,G=0.000000,B=0.023868,A=1.000000)"))))))

(event EventTick
  (params (DeltaSeconds :type Float%20%28single-precision%29))
  (bind _returnvalue (Game|Player|GetPlayerPawn 0))
  (bind _returnvalue_2 (AI|GetBlackboard 0))
  (bind _target (Variables|Default|GetTarget))
  (bind _controlledchar (Variables|Default|GetControlledChar))
  (|CallParentFunction DeltaSeconds)
  (Utilities|IsValid _controlledchar
    (:Is%20Valid
      (if (not (Variables|/Game/_Blueprints/Characters/BP_BaseCharacter.BP_BaseCharacter_C|GetDead _controlledchar))
        (Utilities|FlowControl|Sequence
          (:then_0
            ;[1 1 1] Set wanted location
            (Utilities|IsValid _returnvalue
              (:Is%20Valid
                (Utilities|IsValid _returnvalue_2
                  (:Is%20Valid
                    (AI|Components|Blackboard|SetValueasVector _returnvalue_2 (Utilities|Name|MakeLiteralName "WantedPosition") (Transformation|GetActorLocation _returnvalue)))
                  (:Is%20Not%20Valid
                    (Development|PrintString "Error: Invalid Blackboard" true true "(R=1.000000,G=0.000000,B=0.023868,A=1.000000)"))))))
          (:then_1
            (if (<= (Variables|Default|GetCurrentAttackCooldown) 0.0)
              (Utilities|IsValid _target
                (:Is%20Valid
                  (if (< (Math|Vector|VectorLength (- (Transformation|GetActorLocation _target) (Transformation|GetActorLocation (Variables|Default|GetControlledChar)))) (Variables|Default|GetWantedAttackRange))
                    (CallFunction|MakeMeleeAttack "0, 0, 0")
                    (Variables|Default|SetCurrentAttackCooldown (Variables|Default|GetAttackCooldown))))))))))
    (:Is%20Not%20Valid
      (CallFunction|SetControlledChar))))

(fn ConstructionScript
  (|CallParentFunction))