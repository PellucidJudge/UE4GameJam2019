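; Base AI controller for ranged enemies that runs their behavior tree and targets the player pawn.
; Each tick, while the enemy is alive, it writes the player's position to the blackboard and passes the target to the controlled character.
; A WorldStatic sphere trace from the shoot origin detects cover: blocked shots clear WantToAttack and set half cooldown.
; Clear shots set WantToAttack and trigger Attack1 whenever the cooldown is spent.
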(event Custom|MakeRangeAttack
  (bind _rangecharref (Variables|Default|GetRangeCharRef))
  (Utilities|IsValid _rangecharref
    (:Is%20Valid
      (Default|Attack1 _rangecharref))))

(event EventBeginPlay
  (bind _returnvalue (AI|GetBlackboard 0))
  (bind _returnvalue_2 (Game|Player|GetPlayerPawn 0))
  (|CallParentFunction)
  (Class|AIController|UseBlackboard "/Game/_Blueprints/AI/BB_RangeEnemy.BB_RangeEnemy")
  (AI|RunBehaviorTree "/Game/_Blueprints/AI/BT_RangeEnemy.BT_RangeEnemy")
  (Utilities|IsValid _returnvalue_2
    (:Is%20Valid
      (Variables|Default|SetTarget _returnvalue_2)
      (Utilities|IsValid _returnvalue
        (:Is%20Valid
          (AI|Components|Blackboard|SetValueasObject _returnvalue (Utilities|Name|MakeLiteralName (Variables|Default|GetBBKey_Target)) _returnvalue_2))
        (:Is%20Not%20Valid
          (Development|PrintString "Error: Invalid Blackboard" true true "(R=1.000000,G=0.000000,B=0.023868,A=1.000000)"))))))

(event EventTick
  (params (DeltaSeconds :type Float%20%28single-precision%29))
  (bind _returnvalue (Game|Player|GetPlayerPawn 0))
  (bind _rangecharref (Variables|Default|GetRangeCharRef))
  (bind _rangecharref_2 (Variables|Default|GetRangeCharRef))
  (bind _returnvalue_2 (Transformation|GetActorLocation _returnvalue))
  (|CallParentFunction DeltaSeconds)
  (Utilities|IsValid _rangecharref_2
    (:Is%20Valid
      (if (not (Variables|/Game/_Blueprints/Characters/BP_BaseCharacter.BP_BaseCharacter_C|GetDead _rangecharref_2))
        (Utilities|FlowControl|Sequence
          (:then_0
            ;[1 1 1] Set wanted location
            (Utilities|IsValid _returnvalue
              (:Is%20Valid
                (Utilities|IsValid (AI|GetBlackboard 0)
                  (:Is%20Valid
                    (AI|Components|Blackboard|SetValueasVector (AI|GetBlackboard 0) (Utilities|Name|MakeLiteralName "WantedPosition") _returnvalue_2)
                    (bind _hit (CallFunction|CheckLineOfSight _returnvalue_2 3e+01))
                    (if _hit
                      (AI|Components|Blackboard|SetValueasBool (AI|GetBlackboard 0) (Utilities|Name|MakeLiteralName "WantToAttack") false)
                      (Variables|Default|SetCurrentAttackCooldown (/ (Variables|Default|GetAttackCooldown) 2.0))
                      (else
                        (AI|Components|Blackboard|SetValueasBool (AI|GetBlackboard 0) (Utilities|Name|MakeLiteralName "WantToAttack") true)
                        (if (<= (Variables|Default|GetCurrentAttackCooldown) 0.0)
                          (CallFunction|MakeRangeAttack)
                          (Variables|Default|SetCurrentAttackCooldown (Variables|Default|GetAttackCooldown))))))
                  (:Is%20Not%20Valid
                    (Development|PrintString "Error: Invalid Blackboard" true true "(R=1.000000,G=0.000000,B=0.023868,A=1.000000)"))))))
          (:then_1
            (Utilities|IsValid _rangecharref
              (:Is%20Valid
                (Variables|/Game/_Blueprints/Characters/Enemies/BP_Enemy_RangeBase.BP_Enemy_RangeBase_C|SetTarget _rangecharref (Variables|Default|GetTarget))))))))
    (:Is%20Not%20Valid
      (CallFunction|SetControlledChar))))

(event EventSetControlledChar
  (bind _returnvalue (Pawn|GetControlledPawn))
  (Utilities|IsValid _returnvalue
    (:Is%20Valid
      (bind _asbp_enemy_range_base (Utilities|Casting|CastToBP_Enemy_RangeBase _returnvalue))
      (Variables|Default|SetRangeCharRef _asbp_enemy_range_base))))

(fn ConstructionScript
  (|CallParentFunction))

(fn CheckLineOfSight
  (params (TargetLocation :type Vector) (Radius :type Float%20%28single-precision%29))
  (bind _location (Default|GetShootOrigin (Variables|Default|GetRangeCharRef)))
  (bind _returnvalue (Collision|SphereTraceForObjects _location TargetLocation Radius (Utilities|Array|MakeArray "ObjectTypeQuery1") false 0 "None"))
  (return _returnvalue))