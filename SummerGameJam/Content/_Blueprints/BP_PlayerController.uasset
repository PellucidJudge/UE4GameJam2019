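; Player controller that caches the possessed BP_PlayerCharacter on BeginPlay, sets starting energy, and routes shoot, aim and dash input.
; Aim and dash forward to the character's own functions.
; Shoot looks up the current shot type in DT_ShotData by matching each row's enum, then spawns that row's actor class at the character, facing control rotation.
; The spawned projectile receives the row's damage and the character as owner.
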(event Custom|SetControlledChar
  (bind _returnvalue (Pawn|GetControlledPawn))
  (Utilities|IsValid _returnvalue
    (:Is%20Valid
      (bind _asbp_player_character (Utilities|Casting|CastToBP_PlayerCharacter _returnvalue))
      (Variables|Default|SetControlledChar _asbp_player_character))))

(event EventBeginPlay
  (Variables|Default|SetCurrentEnergy (Variables|Default|GetStartEnergy))
  (CallFunction|SetControlledChar))

(event Input|ActionEvents|InputActionShoot
  (params (Key :type Key%20Structure))
  (bind _controlledchar (Variables|Default|GetControlledChar))
  (:Pressed
    (Utilities|IsValid (Variables|Default|GetControlledChar)
      (:Is%20Valid
        (bind (_success _rowdata) (CallFunction|GetShotDataRow (Variables|Default|GetCurrentShotType)))
        (if _success
          (if (Utilities|IsValidClass (.ActorClass (Utilities|Struct|BreakS_ShotData _rowdata)))
            (bind _returnvalue (Game|SpawnActorfromClass (.ActorClass (Utilities|Struct|BreakS_ShotData _rowdata)) (Math|Transform|MakeTransform (Transformation|GetActorLocation _controlledchar) (Pawn|GetControlRotation :!class /Script/Engine.Controller)) "Undefined" 0 0))
            (Default|SetupProjectile _returnvalue (.Damage (Utilities|Struct|BreakS_ShotData _rowdata)))
            (Actor|SetOwner _returnvalue _controlledchar)
            (else
              (Development|PrintString "Error: Invalid class" true true "(R=1.000000,G=0.000000,B=0.043706,A=1.000000)")))
          (else
            (Development|PrintString "Error: Shot type not found" true true "(R=1.000000,G=0.000000,B=0.043706,A=1.000000)")))))))

(event Input|ActionEvents|InputActionAim
  (params (Key :type Key%20Structure))
  (bind _controlledchar (Variables|Default|GetControlledChar))
  (:Pressed
    (Default|StartAiming _controlledchar))
  (:Released
    (Default|StopAiming _controlledchar)))

(event Input|ActionEvents|InputActionDash
  (params (Key :type Key%20Structure))
  (:Pressed
    (Default|Dash (Variables|Default|GetControlledChar))))

(fn ConstructionScript)

(fn GetShotDataRow
  (params (ShotType :type E_ShotTypes%20Enum :default "NewEnumerator0"))
  (bind _outrownames (DataTable|GetDataTableRowNames "/Game/_Blueprints/DataTables/DT_ShotData.DT_ShotData"))
  (bind _array_element (Utilities|Array|ForEachLoopwithBreak _outrownames :!label _label)
    (:LoopBody
      (bind _returnvalue (Utilities|GetDataTableRow "/Game/_Blueprints/DataTables/DT_ShotData.DT_ShotData" _array_element)
        (:then
          (if (Utilities|Enum|Equal(Enum) ShotType (.Enum (Utilities|Struct|BreakS_ShotData _returnvalue)))
            (LocalVariables|SetLocal_DataTableRowData _returnvalue)
            (LocalVariables|SetLocal_Success true)
            (goto _label Break)))))
    (:Completed
      (return (LocalVariables|GetLocal_Success) (LocalVariables|GetLocal_DataTableRowData)))))