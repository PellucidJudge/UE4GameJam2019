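; Base Blueprint for ranged enemies that attack by firing projectiles.
; When an attack executes and the enemy is alive, it spawns a Projectile at the ShootOrigin component, sets it up and makes itself the owner.
; The shot aims at the Target's root location, or along the capsule's forward vector when no valid Target exists.
; GetShootOrigin returns that component's world location.
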(event EventBeginPlay
  (|CallParentFunction) ; This node is disabled and will not be called.\nDrag off pins to build functionality.
)

(event Collision|EventActorBeginOverlap
  (params (OtherActor :type Actor%20Object%20Reference))
  (|CallParentFunction OtherActor) ; This node is disabled and will not be called.\nDrag off pins to build functionality.
)

(event EventTick
  (params (DeltaSeconds :type Float%20%28single-precision%29))
  (|CallParentFunction DeltaSeconds) ; This node is disabled and will not be called.\nDrag off pins to build functionality.
)

(event EventAttack1
  (|CallParentFunction))

(event EventExecuteAttack
  (bind _shootorigin (Variables|Default|GetShootOrigin))
  (bind _returnvalue (Transformation|GetWorldLocation _shootorigin))
  (if (not (Variables|Default|GetDead))
    (Utilities|IsValid (Variables|Default|GetTarget)
      (:Is%20Valid
        (bind _returnvalue_2 (Game|SpawnActorfromClass (Variables|Default|GetProjectile) (Math|Transform|MakeTransform _returnvalue (Math|Rotator|MakeRotfromX (Math|Vector|Normalize (- (Transformation|GetWorldLocation (Variables|/Script/Engine.Actor|GetRootComponent (Variables|Default|GetTarget))) _returnvalue)))) "AlwaysSpawn" 0 0))
        (Default|SetupProjectile _returnvalue_2 5e+01)
        (Actor|SetOwner _returnvalue_2 self))
      (:Is%20Not%20Valid
        (bind _returnvalue_3 (Game|SpawnActorfromClass (Variables|Default|GetProjectile) (Math|Transform|MakeTransform (Transformation|GetWorldLocation (Variables|Default|GetShootOrigin)) (Math|Rotator|MakeRotfromX (Math|Vector|GetForwardVector (Variables|Default|GetCapsuleComponent)))) "AlwaysSpawn" 0 0))
        (Default|SetupProjectile _returnvalue_3 5e+01)
        (Actor|SetOwner _returnvalue_3 self)))))

(fn ConstructionScript
  (|CallParentFunction))

(fn GetShootOrigin
  (return (Transformation|GetWorldLocation (Variables|Default|GetShootOrigin))))