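; Base Blueprint for melee enemies that supplies the damage step of their attack.
; ExecuteAttack, skipped when dead, runs a debug-enabled box trace just in front of the enemy against pawns and destructibles.
; Hit actors that are not BP_EnemyBase receive fixed damage through I_HealthInterface, so enemies do not hurt each other.
; Attack1 only forwards to the parent, and BeginPlay, overlap and Tick are disabled stubs.
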(event EventBeginPlay
  (|CallParentFunction) ; This node is disabled and will not be called.\nDrag off pins to build functionality.
)

(event Collision|EventActorBeginOverlap
  (params (OtherActor :type Actor%20Object%20Reference))
  (|CallParentFunction OtherActor) ; This node is disabled and will not be called.\nDrag off pins to build functionality.
)

(event EventTick
  (params (DeltaSeconds :type Float%20%28single-precision%29))
  (|CallParentFunction DeltaSeconds) ; This node is disabled and will not be called.\nDrag off pins to build functionality.
)

(event EventAttack1
  (|CallParentFunction))

(event EventExecuteAttack
  (bind _returnvalue (Transformation|GetActorLocation))
  (bind _capsulecomponent (Variables|Default|GetCapsuleComponent))
  (bind _returnvalue_2 (Math|Vector|GetForwardVector _capsulecomponent))
  (bind _returnvalue_3 (* _returnvalue_2 1e+02))
  (bind _returnvalue_4 (+ _returnvalue _returnvalue_3))
  (if (not (Variables|Default|GetDead))
    (bind _uniquehitactors (CallFunction|DamageBox _returnvalue_4 (+ _returnvalue_4 "0, 0,-1.000000") "80.000000,120.000000,50.000000" (Math|Rotator|MakeRotfromX (Math|Vector|GetForwardVector (Variables|Default|GetCapsuleComponent))) (Utilities|Array|MakeArray "ObjectTypeQuery3" "ObjectTypeQuery6") (Utilities|Array|MakeArray self) true))
    (for _array_element _uniquehitactors
      (Utilities|Casting|CastToBP_EnemyBase _array_element
        (:CastFailed
          (if (Utilities|DoesObjectImplementInterface _array_element "/Game/_Blueprints/Interfaces/I_HealthInterface.I_HealthInterface_C")
            (Class|IHealthInterface|HealthDamage(Message) _array_element 4e+01 self "/Script/Engine.DamageType" false false "0, 0, 0")))))))

(fn ConstructionScript
  (|CallParentFunction))