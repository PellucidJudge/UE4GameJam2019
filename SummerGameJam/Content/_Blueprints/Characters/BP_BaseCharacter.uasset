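; BP_BaseCharacter is a base character handling health, death and movement speed, with hit and headshot sounds played through the wave-defence game mode.
; Damage and capped healing adjust health, and death destroys the actor.
; Each tick sets walk speed or curve-scaled running acceleration, passed through CalcMoveModifiers, whose multiplier formula is unconnected, into MaxWalkSpeed.
; DamageBox box-traces and returns unique hit actors without applying damage.
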(event Custom|Death
  ;[1 1 1] Death
  (Variables|Default|SetDead true)
  (Actor|DestroyActor))

(event EventBeginPlay
  (Variables|Health|SetCurrentHealth (Variables|Health|GetMaxHealth)))

(event EventHealthDamage
  (params (Amount :type Float%20%28single-precision%29) (Instigator :type Actor%20Object%20Reference) (DamageType :type Damage%20Type%20Class%20Reference) (HeadShot :type Boolean))
  (bind _returnvalue (Transformation|GetActorLocation))
  ;[1 1 1] Damage
  (if (not (Variables|Default|GetDead))
    (Utilities|FlowControl|Sequence
      (:then_0
        (Development|PrintString "Hello")
        (bind _output_get (Variables|Health|SetCurrentHealth (- (Variables|Health|GetCurrentHealth) Amount)))
        (if (<= _output_get 0.0)
          (CallFunction|Death)))
      (:then_1
        (bind _asbp_game_mode_wave_defence (Utilities|Casting|CastToBP_GameModeWaveDefence (Game|GetGameMode)))
        (if HeadShot
          (Default|GameModePlaySoundatLocation _asbp_game_mode_wave_defence (Variables|Default|GetHeadShotSound) _returnvalue)
          (else
            (Default|GameModePlaySoundatLocation _asbp_game_mode_wave_defence (Variables|Default|GetHitSound) _returnvalue)))))))

(event EventHealthHeal
  (params (Amount :type Float%20%28single-precision%29) (Instigator :type Actor%20Object%20Reference))
  ;[1 1 1] Healing
  (Variables|Health|SetCurrentHealth (Math|Float|Min(Float) (+ (Variables|Health|GetCurrentHealth) Amount) (Variables|Health|GetMaxHealth))))

(event EventTick
  (params (DeltaSeconds :type Float%20%28single-precision%29))
  (CallFunction|UpdateMoveSpeed))

(fn ConstructionScript)

(fn UpdateMoveSpeed
  (bind _walkspeed (Variables|MoveSpeed|GetWalkSpeed))
  (Utilities|FlowControl|Sequence
    (:then_0
      (switch Utilities|FlowControl|Switch|SwitchonE_MovementMode (Variables|MoveSpeed|GetCurrentMovementMode)
        (:NewEnumerator0
          (Variables|MoveSpeed|SetCurrentMoveSpeed (Variables|MoveSpeed|GetWalkSpeed)))
        (:NewEnumerator1
          (Utilities|FlowControl|Sequence
            (:then_1
              (bind _output_get (Variables|MoveSpeed|SetCurrentMoveSpeed (Math|Float|Min(Float) (+ (Variables|MoveSpeed|GetCurrentMoveSpeed) (* (* (Variables|MoveSpeed|GetRunning_Acceleration) (Utilities|Time|GetWorldDeltaSeconds)) (Math|Curves|GetFloatValue (Variables|MoveSpeed|GetRunAccCurve) (/ (- (Variables|MoveSpeed|GetCurrentMoveSpeed) _walkspeed) (- (Variables|MoveSpeed|GetRunSpeed) _walkspeed))))) (Variables|MoveSpeed|GetRunSpeed))))
              (Development|PrintString (Utilities|String|ToString(Float) _output_get) true true "(R=0.000000,G=1.000000,B=0.008637,A=1.000000)" 0.0))))))
    (:then_1
      (Variables|/Script/Engine.CharacterMovementComponent|SetMaxWalkSpeed (Variables|Character|GetCharacterMovement) (Utilities|CalcMoveModifiers (Variables|MoveSpeed|GetCurrentMoveSpeed))))))

(fn DamageBox
  (params (Start :type Vector) (End :type Vector) (HalfSize :type Vector) (Orientation :type Rotator) (ObjectTypes :type Array%20of%20EObjectTypeQuery%20Enums :default "ObjectTypeQuery1") (ActorsToIgnore :type Array%20of%20Actor%20Object%20References) (DebugEnabled :type Boolean))
  (bind _outhits (Class|KismetSystemLibrary|BoxTraceMultiforObjects Start End HalfSize Orientation ObjectTypes false ActorsToIgnore (select DebugEnabled "ForDuration" "None") true))
  (for _array_element _outhits
    (Utilities|Array|AddUnique (LocalVariables|GetLocal_UniqueHitActors) (.HitActor (Collision|BreakHitResult _array_element))))
  (return (LocalVariables|GetLocal_UniqueHitActors)))