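; Railgun projectile that hits instantly along a piercing line and lingers as a fading light until its timeline destroys it.
; On first Tick, a line trace finds world geometry up to a maximum range, then a multi-sphere trace sweeps to that point.
; Health-interface hits take damage and horizontal knockback, doubled damage for head physical material; blocking hits without the interface destroy the projectile.
; The DamagedActors duplicate-hit check is disconnected.
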(event EventBeginPlay
  (|CallParentFunction)
  (Utilities|FlowControl|Sequence
    (:then_0
      (Variables|Default|SetStartIntensity (Variables|/Script/Engine.LightComponentBase|GetIntensity (Variables|Default|GetPointLight))))
    (:then_1
      (bind _newtrack_0 (Timeline|DeletionTimeline PlayFromStart)
        (:Update
          (Rendering|Components|Light|SetIntensity (Variables|Default|GetPointLight) (* (Variables|Default|GetStartIntensity) _newtrack_0)))
        (:Finished
          (Actor|DestroyActor))))))

(event Collision|EventActorBeginOverlap
  (params (OtherActor :type Actor%20Object%20Reference)))

(event EventTick
  (params (DeltaSeconds :type Float%20%28single-precision%29))
  (bind _returnvalue (Components|GetOwner))
  (bind _returnvalue_2 (Components|GetOwner))
  (bind _damage (Variables|Default|GetDamage))
  (Utilities|FlowControl|DoOnce false
    (:Completed
      (bind _newparam (CallFunction|GetRailGunEnd))
      (bind _outhits (Collision|MultiSphereTraceForObjects (Transformation|GetActorLocation) _newparam 5.0 (Utilities|Array|MakeArray "ObjectTypeQuery7" "ObjectTypeQuery6") false (Utilities|Array|MakeArray (Components|GetOwner)) "None"))
      (for _array_element _outhits
        (Utilities|IsValid _returnvalue
          (:Is%20Valid
            (if (Utilities|DoesObjectImplementInterface (.HitActor (Collision|BreakHitResult _array_element)) "/Game/_Blueprints/Interfaces/I_HealthInterface.I_HealthInterface_C")
              (switch string (Utilities|GetDisplayName (.PhysMat (Collision|BreakHitResult _array_element)))
                (:PM_Body
                  (Class|IHealthInterface|HealthDamage(Message) (.HitActor (Collision|BreakHitResult _array_element)) _damage _returnvalue_2 "/Script/Engine.DamageType" false true (Math|Vector|Normalize (Math|Vector|MakeVector (.x (- (.Location (Collision|BreakHitResult _array_element)) (Transformation|GetActorLocation _returnvalue))) (.y (- (.Location (Collision|BreakHitResult _array_element)) (Transformation|GetActorLocation _returnvalue))) 0.0))))
                (:PM_Head
                  (Class|IHealthInterface|HealthDamage(Message) (.HitActor (Collision|BreakHitResult _array_element)) (* _damage 2.0) _returnvalue_2 "/Script/Engine.DamageType" true true (Math|Vector|Normalize (Math|Vector|MakeVector (.x (- (.Location (Collision|BreakHitResult _array_element)) (Transformation|GetActorLocation _returnvalue))) (.y (- (.Location (Collision|BreakHitResult _array_element)) (Transformation|GetActorLocation _returnvalue))) 0.0)))))
              (elif (.bBlockingHit (Collision|BreakHitResult _array_element))
                (Actor|DestroyActor)))))))))

(event EventSetupProjectile
  (params (Damage :type Float%20%28single-precision%29))
  (|CallParentFunction Damage))

(fn ConstructionScript
  (|CallParentFunction))

(fn GetRailGunEnd
  (bind _returnvalue (Transformation|GetActorLocation))
  (bind (_outhit _returnvalue_2) (Collision|LineTraceForObjects _returnvalue (+ _returnvalue (* (Math|Vector|GetForwardVector (Variables|Default|GetDefaultSceneRoot)) 1e+04)) (Utilities|Array|MakeArray "ObjectTypeQuery1") false (Utilities|Array|MakeArray (Components|GetOwner)) "None"))
  (if _returnvalue_2
    (return (.ImpactPoint (Collision|BreakHitResult _outhit)))
    (else
      (return (.TraceEnd (Collision|BreakHitResult _outhit))))))