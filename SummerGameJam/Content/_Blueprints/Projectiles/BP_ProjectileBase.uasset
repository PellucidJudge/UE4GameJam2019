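; BP_ProjectileBase is a base projectile Blueprint that deals damage to actors implementing the health interface.
; A SetupProjectile event sets its damage amount.
; Each tick it sphere-traces at its location with the collision radius, ignoring its owner, and sends a health damage message to a qualifying hit actor.
; It destroys itself only after such a hit, so other hit objects do not stop it in this graph.
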(event Custom|SetupProjectile
  (params (Damage :type Float%20%28single-precision%29))
  (Variables|Default|SetDamage Damage))

(event EventBeginPlay)

(event EventTick
  (params (DeltaSeconds :type Float%20%28single-precision%29))
  (bind _returnvalue (Transformation|GetActorLocation))
  (bind _outhit (Collision|SphereTraceForObjects _returnvalue (+ _returnvalue "0, 0,1.000000") (Components|Sphere|GetScaledSphereRadius (Variables|Default|GetCollision)) (Utilities|Array|MakeArray "ObjectTypeQuery3" "ObjectTypeQuery1" "ObjectTypeQuery6") false (Utilities|Array|MakeArray (Components|GetOwner)) "None"))
  (if (Utilities|DoesObjectImplementInterface (.HitActor (Collision|BreakHitResult _outhit)) "/Game/_Blueprints/Interfaces/I_HealthInterface.I_HealthInterface_C")
    (Class|IHealthInterface|HealthDamage(Message) (.HitActor (Collision|BreakHitResult _outhit)) (Variables|Default|GetDamage) (Components|GetOwner) "/Script/Engine.DamageType")
    (Actor|DestroyActor)))

(fn ConstructionScript)