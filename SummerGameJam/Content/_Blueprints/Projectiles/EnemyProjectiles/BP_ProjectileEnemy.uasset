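; Enemy projectile Blueprint whose only active gameplay logic is a CheckForHit function, with its event graph left at disabled defaults.
; CheckForHit sphere-traces at the actor's location using the Collision radius, against WorldStatic, Destructible and one custom object type, ignoring the owner.
; It returns the hit result and prints a leftover debug "Hello" whenever the trace hits.
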(event EventBeginPlay
  (|CallParentFunction) ; This node is disabled and will not be called.\nDrag off pins to build functionality.
)

(event Collision|EventActorBeginOverlap
  (params (OtherActor :type Actor%20Object%20Reference)))

(event EventTick
  (params (DeltaSeconds :type Float%20%28single-precision%29))
  (|CallParentFunction DeltaSeconds) ; This node is disabled and will not be called.\nDrag off pins to build functionality.
)

(fn ConstructionScript
  (|CallParentFunction))

(fn CheckforHit
  (bind _returnvalue (Transformation|GetActorLocation))
  (bind (_outhit _returnvalue_2) (Collision|SphereTraceForObjects _returnvalue (+ _returnvalue "0, 0,1.000000") (Components|Sphere|GetScaledSphereRadius (Variables|Default|GetCollision)) (Utilities|Array|MakeArray "ObjectTypeQuery8" "ObjectTypeQuery1" "ObjectTypeQuery6") false (Utilities|Array|MakeArray (Components|GetOwner)) "None"))
  (Utilities|FlowControl|Sequence
    (:then_0
      (if _returnvalue_2
        (Development|PrintString "Hello")))
    (:then_1
      (return _outhit))))