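; Spread-shot projectile that, on setup, spawns extra pellet projectiles to form a randomized spread, like a shotgun blast.
; SetupProjectile stores Damage, then spawns AdditionalShotsCount BP_Projectile_SpreadShotAdds at its own location, passing each valid one the same Damage.
; Each pellet's rotation offsets the forward pitch and yaw by Spread scaled with randomized, normalized 2D vector components; roll is also derived from pitch.
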(event EventBeginPlay
  (|CallParentFunction) ; This node is disabled and will not be called.\nDrag off pins to build functionality.
)

(event Collision|EventActorBeginOverlap
  (params (OtherActor :type Actor%20Object%20Reference)))

(event EventTick
  (params (DeltaSeconds :type Float%20%28single-precision%29))
  (|CallParentFunction DeltaSeconds) ; This node is disabled and will not be called.\nDrag off pins to build functionality.
)

(event EventSetupProjectile
  (params (Damage :type Float%20%28single-precision%29))
  (bind _returnvalue (Math|Random|RandomFloatinRange -1.0 1.0))
  (bind _returnvalue_2 (Math|Random|RandomFloatinRange -1.0 1.0))
  (bind _returnvalue_3 (Math|Random|RandomFloatinRange -1.0 1.0))
  (bind _defaultsceneroot (Variables|Default|GetDefaultSceneRoot))
  (bind _spread (Variables|Default|GetSpread))
  (bind _returnvalue_4 (Math|Vector|GetForwardVector _defaultsceneroot))
  (bind _returnvalue_5 (Math|Vector|MakeVector _returnvalue _returnvalue_2 0.0))
  (bind _returnvalue_6 (Math|Rotator|MakeRotfromX _returnvalue_4))
  (bind _returnvalue_7 (Math|Vector|Normalize _returnvalue_5))
  (bind _returnvalue_8 (* (.x _returnvalue_7) _returnvalue_3))
  (bind _returnvalue_9 (* _spread _returnvalue_8))
  (bind _returnvalue_10 (+ (.pitch _returnvalue_6) _returnvalue_9))
  (Variables|Default|SetDamage Damage)
  (for _index (range 1 (Variables|Default|GetAdditionalShotsCount))
    (bind _returnvalue_11 (Game|SpawnActorfromClass "/Game/_Blueprints/Projectiles/BP_Projectile_SpreadShotAdds.BP_Projectile_SpreadShotAdds_C" (Math|Transform|MakeTransform (Transformation|GetActorLocation) (Math|Rotator|MakeRotator _returnvalue_10 _returnvalue_10 (+ (.yaw _returnvalue_6) (* _spread (* (.y _returnvalue_7) (Math|Random|RandomFloatinRange -1.0 1.0)))))) "Undefined" 0 0))
    (Utilities|IsValid _returnvalue_11
      (:Is%20Valid
        (Default|SetupProjectile _returnvalue_11 Damage)))))

(fn ConstructionScript
  (|CallParentFunction))